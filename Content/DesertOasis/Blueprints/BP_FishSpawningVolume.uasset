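; Box volume that populates the desert oasis level with wandering AI fish, sized in the construction script from BoxExtents.
; On BeginPlay it spawns BP_FishAI actors at random points inside, passes each the bounds, stores them in FishArray and calls MoveFIsh after every spawn.
; MoveFIsh loops over the whole array, calling SpawnDefaultController and AIMoveTo random in-box points, then re-triggers itself on success or through a delay.
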(event `self.ReceiveBeginPlay`
  (bind _box_extents (`self.Box Extents`))
  ;[1 1 1] Spawn FishAI inside box extents volume
  (for _ (range (+ (`self.Max Fish`) 1))
    (bind _returnvalue (`|SpawnActorFromClass` "/Game/DesertOasis/Blueprints/BP_FishAI.BP_FishAI_C" (`KismetMathLibrary.MakeTransform` (`KismetMathLibrary.RandomPointInBoundingBox` (`SceneComponent.K2_GetComponentLocation` (`self.Scene`)) _box_extents)) "Undefined" "OverrideRootScale"))
    ;[1 1 1] Add FishAI to an array to access later
    (`KismetArrayLibrary.Array_Add` (`self.FishArray`) _returnvalue)
    (set `/Game/DesertOasis/Blueprints/BP_FishAI.BoxOrigin` (`SceneComponent.K2_GetComponentLocation` (`self.Scene`)) _returnvalue)
    (set `/Game/DesertOasis/Blueprints/BP_FishAI.BoxExtent` _box_extents _returnvalue)
    (`self.MoveFIsh`)))

(event `MoveFIsh`
  ;[1 1 1] Randomly moves the FishAI to a location within the box extents
  (for _array_element (`self.FishArray`)
    (`Pawn.SpawnDefaultController` _array_element)
    (`|AIMoveTo` (`Pawn.GetController` _array_element) null (`KismetMathLibrary.RandomPointInBoundingBox` (`SceneComponent.K2_GetComponentLocation` (`self.Scene`)) (`self.Box Extents`))
      (:`then`
        ;;[1 1 1] Move the FishAI after 10 seconds if it has not reached its destination
        (`KismetSystemLibrary.Delay` 10.0))
      (:`OnSuccess`
        _))
    (`self.MoveFIsh`)))

(fn `UserConstructionScript`
  (`BoxComponent.SetBoxExtent` (`self.Box`) (`self.Box Extents`) true))