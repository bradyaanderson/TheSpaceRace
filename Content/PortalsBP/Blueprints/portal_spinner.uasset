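; Portal spinner actor that carries two child-actor PortalBP portals and continuously rotates them.
; The construction script links the two portals as each other's TargetPortal.
; BeginPlay turns off AllowRecursionCamera on both portals.
; Tick adds a fixed local yaw step each frame without delta-time scaling, so spin speed depends on frame rate.
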(event `self.ReceiveBeginPlay`
  (`|ExecutionSequence`
    (:`then_0`
      (bind _asportal_bp (cast `/Game/PortalsBP/Blueprints/PortalBP` (`ChildActorComponent.ChildActor` (`self.ChildActor`))))
      (set `/Game/PortalsBP/Blueprints/PortalBP.AllowRecursionCamera` false _asportal_bp))
    (:`then_1`
      (bind _asportal_bp_2 (cast `/Game/PortalsBP/Blueprints/PortalBP` (`ChildActorComponent.ChildActor` (`self.ChildActor1`))))
      (set `/Game/PortalsBP/Blueprints/PortalBP.AllowRecursionCamera` false _asportal_bp_2))))

(event `self.ReceiveTick`
  (params (DeltaSeconds :type "Float (single-precision)"))
  (`self.K2_AddActorLocalRotation` (`KismetMathLibrary.MakeRotator` 0.0 0.0 1.0)))

(fn `UserConstructionScript`
  (bind _asportal_bp (cast `/Game/PortalsBP/Blueprints/PortalBP` (`ChildActorComponent.ChildActor` (`self.ChildActor`))))
  (bind _asportal_bp_2 (cast `/Game/PortalsBP/Blueprints/PortalBP` (`ChildActorComponent.ChildActor` (`self.ChildActor1`))))
  (set `/Game/PortalsBP/Blueprints/PortalBP.TargetPortal` _asportal_bp_2 _asportal_bp)
  (set `/Game/PortalsBP/Blueprints/PortalBP.TargetPortal` _asportal_bp _asportal_bp_2))